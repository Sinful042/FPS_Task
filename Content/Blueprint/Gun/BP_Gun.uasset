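; BP_Gun is a data-driven gun actor that fires projectiles and plays a reload animation.
; The construction script loads the GunName row from DT_Guns, setting the mesh and snapping GunBarrel to its socket.
; FireEvent plays a sound and spawns a damage-carrying projectile at the barrel, while ReleodEvent holds a Releod flag during the montage.
; AttachPlayer snaps the gun to a socket on the parent actor's "ArmMesh"-tagged mesh.
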(event Custom|ReleodEvent
  ;[1 1 1] Releod Event
  (Variables|Default|SetReleod true)
  (Animation|Montage|PlayMontage (Variables|Default|GetSkeletalMesh) (.releodanimmontage (Variables|Default|GetST_GunProperties))
    (:OnCompleted
      _)
    (:OnBlendOut
      _)
    (:OnInterrupted
      _))
  (Variables|Default|SetReleod false))

(event Custom|FireEvent
  (bind _st_gunproperties (Variables|Default|GetST_GunProperties))
  (bind _gunbarrel (Variables|Default|GetGunBarrel))
  (Audio|PlaySoundatLocation (.firesound _st_gunproperties) (Transformation|GetActorLocation) "0, 0, 0" 1.0 1.0 0.0 0 0 0)
  (Game|SpawnActorfromClass "/Game/FP_Blueprint/Blueprints/DefaultBP/FirstPersonProjectile.FirstPersonProjectile_C" (Math|Transform|MakeTransform (Transformation|GetWorldLocation _gunbarrel) (Transformation|GetWorldRotation _gunbarrel)) "Undefined" 0 (.damage _st_gunproperties) 0))

(event EventBeginPlay)

(event Collision|EventActorBeginOverlap
  (params (OtherActor :type Actor%20Object%20Reference)))

(event EventTick
  (params (DeltaSeconds :type Float%20%28single-precision%29)))

(fn ConstructionScript
  (bind _returnvalue (Utilities|GetDataTableRow "/Game/Blueprint/Gun/DT_Guns.DT_Guns" (Variables|Default|GetGunName))
    (:then
      (Variables|Default|SetST_GunProperties _returnvalue)
      (Class|SkinnedMeshComponent|SetSkeletalMesh (Variables|Default|GetSkeletalMesh) (.sk_gun (Variables|Default|GetST_GunProperties)) true)
      (Transformation|AttachComponentToComponent (Variables|Default|GetGunBarrel) (Variables|Default|GetSkeletalMesh) (.barrelsocketname (Variables|Default|GetST_GunProperties)) "SnapToTarget" "SnapToTarget" "SnapToTarget" true))))

(fn AttachPlayer
  (bind _returnvalue (Actor|GetParentActor))
  (bind _st_gunproperties (Variables|Default|GetST_GunProperties))
  (bind _returnvalue_2 (Actor|GetComponentsbyTag _returnvalue "/Script/Engine.SkeletalMeshComponent" "ArmMesh"))
  (bind _output (Utilities|Array|Get(acopy) _returnvalue_2))
  (Utilities|IsValid _output
    (:Is%20Valid
      (if (Utilities|Array|ContainsItem (Transformation|GetAllSocketNames _output) (.socketname _st_gunproperties))
        (Transformation|AttachComponentToComponent _output (.socketname _st_gunproperties) "SnapToTarget" "SnapToTarget" "SnapToTarget" true)))))