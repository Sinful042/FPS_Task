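; Enemy actor that takes projectile damage and shows a health bar widget.
; On BeginPlay it registers its max health with the EnemyObserver on player 0's FirstPersonCharacter, keeping the returned index, and initializes the bar.
; GetHit acts only on authority, since the projectile is replicated, passing damage to that character's SetEnemyHealth.
; HitDamage subtracts damage from the observer's health array entry and updates the bar.
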(event EventBeginPlay
  (Utilities|FlowControl|Sequence
    (:then_0
      (bind _asfirst_person_character (Utilities|Casting|CastToFirstPersonCharacter (Game|GetPlayerCharacter 0)))
      (bind _output_get (Variables|Default|SetAs%20First%20Person%20Character _asfirst_person_character))
      (bind _output_get_2 (Variables|Default|SetEnemy%20Properties (Variables|/Game/FP_Blueprint/Blueprints/DefaultBP/FirstPersonCharacter.FirstPersonCharacter_C|GetEnemyObserver _output_get)))
      (bind _enemyindex (Default|RegisterEnemy _output_get_2 (Variables|Default|GetMaxHealth)))
      (Variables|Default|SetEnemy%20Index _enemyindex))
    (:then_1
      (bind _aswbp_health_bar (Utilities|Casting|CastToWBP_HealthBar (UserInterface|GetWidget (Variables|Default|GetWidget))))
      (Variables|/Game/Widget/WBP_HealthBar.WBP_HealthBar_C|SetMaxHealth _aswbp_health_bar (Math|Conversions|ToFloat(Integer) (Variables|Default|GetMaxHealth))))))

(event Collision|EventActorBeginOverlap
  (params (OtherActor :type Actor%20Object%20Reference)))

(event EventTick
  (params (DeltaSeconds :type Float%20%28single-precision%29)))

(event EventGetHit
  (params (Damage :type Integer))
  ;[1 1 1] Only  Hit  Damage in Server Because ProjectTile Replicated
  (Networking|SwitchHasAuthority
    (:Authority
      (Default|SetEnemyHealth (Variables|Default|GetAs%20First%20Person%20Character) self Damage))))

(fn ConstructionScript)

(fn HitDamage
  (params (Damage :type Integer))
  (bind _enemy_properties (Variables|Default|GetEnemy%20Properties))
  (bind _enemy_index (Variables|Default|GetEnemy%20Index))
  (bind _enemyhealts (Variables|/Game/Blueprint/Enemy/BP_EnemyObserver.BP_EnemyObserver_C|GetEnemyHealts _enemy_properties))
  (bind _output (Utilities|Array|Get(acopy) _enemyhealts _enemy_index))
  (bind _returnvalue (- _output Damage))
  (Utilities|Array|SetArrayElem (Variables|/Game/Blueprint/Enemy/BP_EnemyObserver.BP_EnemyObserver_C|GetEnemyHealts (Variables|Default|GetEnemy%20Properties)) (Variables|Default|GetEnemy%20Index) _returnvalue)
  (bind _aswbp_health_bar (Utilities|Casting|CastToWBP_HealthBar (UserInterface|GetWidget (Variables|Default|GetWidget))))
  (Default|SetPercent _aswbp_health_bar _returnvalue))